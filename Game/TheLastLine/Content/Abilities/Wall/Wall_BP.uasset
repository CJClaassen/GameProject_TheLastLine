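; Wall ability actor that raises itself out of its spawn height, with a timed despawn branch.
; BeginPlay calls CastAbility with a zero location, which stores CasterLocation and sets RaiseWall.
; While RaiseWall is set, Tick pins X/Y to that location and climbs at RaiseSpeed if RaiseDuration exceeds the frame delta.
; RaiseDuration never decrements and RaiseWall never clears here, so the WallDuration destroy branch is not reached by this graph alone.
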(event EventBeginPlay
  (CallFunction|CastAbility "0, 0, 0"))

(event Collision|EventActorBeginOverlap
  (params (OtherActor :type Actor%20Object%20Reference)))

(event EventTick
  (params (DeltaSeconds :type Float%20%28single-precision%29))
  (bind _casterlocation (Variables|Default|GetCasterLocation))
  (if (Variables|Default|GetraiseWall)
    ;[1 1 1] Raise wall animation
    (Variables|Default|SetActivatedTime (Utilities|Time|GetGameTimeinSeconds))
    (if (> (- (Variables|Default|GetraiseDuration) DeltaSeconds) 0.0)
      (Transformation|SetActorLocation (Math|Vector|MakeVector (.x _casterlocation) (.y _casterlocation) (+ (.z (Transformation|GetActorLocation)) (* DeltaSeconds (Variables|Default|GetRaiseSpeed)))) false false))
    (elif (< (Variables|Default|GetWallDuration) (- (Utilities|Time|GetGameTimeinSeconds) (Variables|Default|GetActivatedTime)))
      (Actor|DestroyActor))))

(event EventCastAbility
  (params (CastLocation :type Vector :default "0, 0, 0"))
  ;[1 1 1] Trigger Wall raise
  (Variables|Default|SetCasterLocation CastLocation)
  (Variables|Default|SetraiseWall true))

(fn ConstructionScript
  (|CallParentFunction))